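; Player Blueprint for a physics-driven auto-runner that moves along Y at constant speed and jumps with a cube-style flip.
; Tick applies strong custom downward acceleration to the Collision body and overwrites its velocity, preserving only Z.
; Enhanced Input jump requires a box-trace hit around the body, then resets vertical velocity and applies an impulse.
; Each jump also starts a timeline that rolls the mesh another quarter turn.
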(event `self.ReceiveBeginPlay`
  (`EnhancedInputSubsystemInterface.AddMappingContext` (pcsubsystem `EnhancedInputLocalPlayerSubsystem` (`GameplayStatics.GetPlayerController` 0)) "/Game/IMC_Player.IMC_Player" 0 (struct)))

(event `self.ReceiveTick`
  (params (DeltaSeconds :type "Float (single-precision)"))
  (bind _collision (`self.Collision`))
  (`PrimitiveComponent.AddForce` (`self.Collision`) (0.0 0.0 -9404.0) "None" true)
  (bind _returnvalue (`PrimitiveComponent.GetPhysicsLinearVelocity` _collision "None"))
  (`PrimitiveComponent.SetPhysicsLinearVelocity` _collision (`KismetMathLibrary.MakeVector` 0.0 (`self.PlayerSpeed`) (.z _returnvalue)) false "None"))

(event `EnhancedInput|/Game/IA_Jump`
  (params (ActionValue :type Boolean) (ElapsedSeconds :type "Float (double-precision)") (TriggeredSeconds :type "Float (double-precision)") (InputAction :type "InputAction Object Reference" :default "/Game/IA_Jump.IA_Jump"))
  (bind _returnvalue (`SceneComponent.K2_GetComponentLocation` (`self.Collision`)))
  (:`Triggered`
    (bind (_outhit _returnvalue_2) (`KismetSystemLibrary.BoxTraceSingle` :`Start` _returnvalue :`End` _returnvalue :`HalfSize` (50.0 50.0 55.0) :`TraceChannel` "TraceTypeQuery1" :`DrawDebugType` "ForOneFrame"))
    (if _returnvalue_2
      (bind _returnvalue_3 (`PrimitiveComponent.GetPhysicsLinearVelocity` (`self.Collision`) "None"))
      (`PrimitiveComponent.SetPhysicsLinearVelocity` (`self.Collision`) (`KismetMathLibrary.MakeVector` (.x _returnvalue_3) (.y _returnvalue_3)) false "None")
      (`PrimitiveComponent.AddImpulse` (`self.Collision`) (`KismetMathLibrary.MakeVector` 0.0 0.0 (`self.JumpVelocity`)) "None" true)
      (set `self.TargetRotation` (+ (`self.TargetRotation`) 90.0))
      (`TimelineComponent.SetPlayRate` (`self.Timeline`) (/ 1.0 (`self.TimeRotation`)))
      (bind (_direction _newtrack_0) (`Timeline|Timeline` :!via `PlayFromStart`)
        (:`Update`
          (`SceneComponent.K2_SetRelativeRotation` (`self.SM_Player`) (`KismetMathLibrary.MakeRotator` (`KismetMathLibrary.Lerp` (- (`self.TargetRotation`) 90.0) (`self.TargetRotation`) _newtrack_0)) false false))))))

(fn `UserConstructionScript`)